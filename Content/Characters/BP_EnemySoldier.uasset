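; Enemy soldier character that runs a behavior tree, can be highlighted by a lock-on widget, and takes damage.
; Pawn sensing passes seen pawns to DetectPawn with the player as target and Melee as state, and the first sighting reveals the health bar tag.
; Damage reduces health in the stats component and plays a hurt animation.
; The component's delegates update the health bar and trigger death handling at zero health.
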(event `self.ReceiveBeginPlay`
  (`AIController.RunBehaviorTree` (`AIBlueprintHelperLibrary.GetAIController` self) "/Game/Characters/AI/BT_EnemySoldier.BT_EnemySoldier")
  (bind _aswbp_enemy_soldier (cast `/Game/UI/WBP_EnemySoldier` (`WidgetComponent.GetUserWidgetObject` (`self.EnemyTag`))))
  (set `self.HealthBar` _aswbp_enemy_soldier))

(event `self.OnSelect`
  (`SceneComponent.SetVisibility` (`self.LockonWidget`) true false))

(event `self.OnDeselect`
  (`SceneComponent.SetVisibility` (`self.LockonWidget`) false false))

(event `self.ReceiveAnyDamage`
  (params (Damage :type "Float (single-precision)") (DamageType :type "DamageType Object Reference") (InstigatedBy :type "Controller Object Reference") (DamageCauser :type "Actor Object Reference"))
  (`StatsComponent.ReduceHealth` (`self.StatsComp`) Damage null)
  (`self.PlayHurtAnim`))

(event `self.PawnSensing.OnSeePawn`
  (params (Pawn :type "Pawn Object Reference"))
  (`self.DetectPawn` Pawn (`GameplayStatics.GetPlayerPawn` 0) "Melee")
  (`/Engine/EditorBlueprintResources/StandardMacros.DoOnce` false
    (:`Completed`
      (`SceneComponent.SetVisibility` (`self.EnemyTag`) true false)
      (`/Game/UI/WBP_EnemySoldier.SetHealth` (`self.HealthBar`) (`StatsComponent.GetStatPercentage` (`self.StatsComp`) "Health" "MaxHealth")))))

(event `self.StatsComp.OnHealthPercentUpdateDelegate`
  (params (Percentage :type "Float (single-precision)"))
  (`/Game/UI/WBP_EnemySoldier.SetHealth` (`self.HealthBar`) Percentage))

(event `self.StatsComp.OnZeroHealthDelegate`
  (`self.HandleDeath`))

(fn `UserConstructionScript`)